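; Enemy base Blueprint with a render-target damage painting prototype for its skeletal mesh; the setup is disconnected and marked not in use.
; That setup creates a damage render target, feeds it to a dynamic material and aims a self-only scene capture at it.
; PaintDamage briefly swaps in an unwrap material with hit location and radius, captures the mesh into the target, then restores the original material.
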(event `self.ReceiveBeginPlay`)

(fn `PaintDamage`
  (params (`Hit Location` :type "Vector Structure") (Radius :type "Float (double-precision)"))
  (bind _skeletalmesh (`self.SkeletalMesh`))
  (`|ExecutionSequence`
    (:`then_0`
      ;[1 1 1] Unwrap and capture
      (set `self.BaseMaterial` (`PrimitiveComponent.GetMaterial` _skeletalmesh 0))
      (`PrimitiveComponent.SetMaterial` _skeletalmesh 0 "/Game/Materials/M_Unwrapper.M_Unwrapper")
      (`MeshComponent.SetVectorParameterValueOnMaterials` _skeletalmesh "CaptureLocation" (`SceneComponent.K2_GetComponentLocation` (`self.DefaultSceneRoot`)))
      (`MeshComponent.SetVectorParameterValueOnMaterials` _skeletalmesh "HitLocation" `Hit Location`)
      (`MeshComponent.SetScalarParameterValueOnMaterials` _skeletalmesh "ImpactRadius" Radius)
      (`SceneCaptureComponent2D.CaptureScene` (`self.SceneCaptureComponent2D`)))
    (:`then_1`
      (`PrimitiveComponent.SetMaterial` (`self.SkeletalMesh`) 0 (`self.BaseMaterial`)))))

(fn `UserConstructionScript`)