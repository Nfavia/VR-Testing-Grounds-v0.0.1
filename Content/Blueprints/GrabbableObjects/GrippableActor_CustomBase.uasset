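; Base actor for VR grabbable objects, handling physics setup, weight classification and grip state.
; On BeginPlay it configures simulation and gravity, classifies weight from mesh mass (with a separate gravity-free class), disables far grabbing for the heaviest class, and caches multi-grip support.
; Tick mirrors the held state into IsGrabbed, and when a VR_Player overlap ends on an unheld object, the mesh blocks the Pawn channel again.
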(event `self.ReceiveBeginPlay`
  ;[0.4142 1 0.3172] Begin Play
  (`self.SeupPhysics`)
  (bind _returnvalue (`VRGripInterface.AllowsMultipleGrips`))
  (set `self.bCanBeMultiGrabbed` _returnvalue))

(event `self.ReceiveTick`
  (params (DeltaSeconds :type "Float (single-precision)"))
  ;[1 0.2864 0.9561] Tick
  (bind (_holdingcontrollers _bisheld) (`VRGripInterface.IsHeld`))
  (set `self.bIsGrabbed` _bisheld))

(event `self.ReceiveActorEndOverlap`
  (params (OtherActor :type "Actor Object Reference"))
  ;[0.237 0.9402 1] Actor End Overlap
  (cast `/Game/Blueprints/Player/VR_Player` OtherActor)
  (if (not (`self.bIsGrabbed`))
    (`PrimitiveComponent.SetCollisionResponseToChannel` (`self.GrippableMeshRoot`) "ECC_Pawn" "ECR_Block")))

(fn `SeupPhysics`
  (locals (fLightWeight :type "Float (double-precision)" :default 5.0) (fMediumWeight :type "Float (double-precision)" :default 22.0))
  (`self.GrippableMeshRoot`
    (:`then`
      (`|ExecutionSequence`
        (:`then_0`
          (`PrimitiveComponent.SetSimulatePhysics` (`self.GrippableMeshRoot`) (`self.bShouldSimulateOnBegin`))
          (if (`self.bAffectedByGravity`)
            (`PrimitiveComponent.SetEnableGravity` (`self.GrippableMeshRoot`) true)
            (if (<= (`PrimitiveComponent.GetMass` (`self.GrippableMeshRoot`)) (`local.fLightWeight`))
              (set `self.ObjectWeightClass` "NewEnumerator1")
              (elif (<= (`PrimitiveComponent.GetMass` (`self.GrippableMeshRoot`)) (`local.fMediumWeight`))
                (set `self.ObjectWeightClass` "NewEnumerator2")
                (elif (> (`PrimitiveComponent.GetMass` (`self.GrippableMeshRoot`)) (`local.fMediumWeight`))
                  (set `self.ObjectWeightClass` "NewEnumerator3"))))
            (else
              (`PrimitiveComponent.SetEnableGravity` (`self.GrippableMeshRoot`) false)
              (set `self.ObjectWeightClass` "NewEnumerator0"))))
        (:`then_1`
          (if (`|EnumEquality` (`self.ObjectWeightClass`) "NewEnumerator3")
            (set `self.bIsFarGrabbable` false)))))
    (:`else`
      (`KismetSystemLibrary.PrintString` (`KismetStringLibrary.Concat_StrStr` (`KismetSystemLibrary.GetObjectName` self) ": Does not have Static Mesh assigned to it.") true true (struct :`R` 1.0 :`G` 0.051168 :`B` 0.09097 :`A` 1.0)))))

(fn `UserConstructionScript`)