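; Grabbable dagger weapon that orients itself while being far-grabbed and leaves bleeding cuts on enemies it touches.
; During a far grab, Tick interpolates the mesh root rotation toward one derived from projectile velocity.
; Blade overlap with a BP_EnemyBase arms damage painting; Tick then box-traces at the blade, spawning attached fading decals and bleed Niagara effects on that enemy.
; An author note marks this painting logic for moving to a weapon base Blueprint.
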(event `self.ReceiveTick`
  (params (DeltaSeconds :type "Float (single-precision)"))
  (bind _bladecollider (`self.BladeCollider`))
  (bind _returnvalue (`KismetMathLibrary.NegateVector` (`self.GetActorUpVector`)))
  (bind _returnvalue_2 (`SceneComponent.K2_GetComponentLocation` _bladecollider))
  (bind (_returnvalue_roll _returnvalue_pitch _returnvalue_yaw) (`KismetMathLibrary.BreakRotator` (`KismetMathLibrary.FindLookAtRotation` _returnvalue (+ _returnvalue (`MovementComponent.Velocity` (`self.ProjectileMovement`))))))
  (`parent.ReceiveTick` DeltaSeconds)
  (`|ExecutionSequence`
    (:`then_0`
      ;[0.005604 0.2472 1] Far Grab Rotation Logic
      (if (`self.IsBeingFarGrabbed`)
        (`SceneComponent.K2_SetWorldRotation` (`self.GrippableMeshRoot`) (`KismetMathLibrary.RInterpTo` (`self.K2_GetActorRotation`) (`KismetMathLibrary.MakeRotator` _returnvalue_roll (- _returnvalue_pitch 90.0) _returnvalue_yaw) DeltaSeconds 50.0) false false)))
    (:`then_1`
      ;[1 1 1] Draw Damage Effect on Enemy (Change this to function on a Weapon Base Blueprint)
      (if (`self.bPaintDamage`)
        (bind _outhit (`KismetSystemLibrary.BoxTraceSingleForObjects` :`Start` _returnvalue_2 :`End` (+ _returnvalue_2 (0.1 0.1 0.1)) :`HalfSize` (/ (`BoxComponent.BoxExtent` _bladecollider) 3.75) :`Orientation` (`SceneComponent.K2_GetComponentRotation` _bladecollider) :`ObjectTypes` (`|MakeArray` "ObjectTypeQuery3" :!type "EObjectTypeQuery Enum") :`TraceColor` (struct :`R` 1.0 :`G` 0.079082 :`B` 0.882619 :`A` 1.0)))
        (bind (_bblockinghit _binitialoverlap _time _distance _location _impactpoint _normal _impactnormal _physmat _hitactor _hitcomponent) (`GameplayStatics.BreakHitResult` _outhit))
        (if (== (`self.Target`) _hitactor)
          (bind _returnvalue_3 (`KismetMathLibrary.Conv_VectorToRotator` _impactnormal))
          (bind _returnvalue_4 (`GameplayStatics.SpawnDecalAttached` (`self.DamageDecal Material`) (`self.DamageDecalSize`) _hitcomponent "None" _impactpoint (`KismetMathLibrary.ComposeRotators` _returnvalue_3 (struct :`Yaw` 90.0)) "KeepWorldPosition"))
          (`DecalComponent.SetFadeOut` _returnvalue_4 0.5 (`self.DamageEffectLifeSpan`) false)
          (`NiagaraFunctionLibrary.SpawnSystemAttached` (`self.BleedFX`) _hitcomponent "None" _impactpoint _returnvalue_3 "KeepWorldPosition" true))))))

(event `self.BladeCollider.OnComponentBeginOverlap`
  (params (OverlappedComponent :type "PrimitiveComponent Object Reference") (OtherActor :type "Actor Object Reference") (OtherComp :type "PrimitiveComponent Object Reference") (OtherBodyIndex :type Integer) (bFromSweep :type Boolean) (SweepResult :type "HitResult Structure (by ref)"))
  ;[1 1 1] Start Painting Damage on Overlap
  (bind _asbp_enemy_base (cast `/Game/Blueprints/Enemies/BP_EnemyBase` OtherActor))
  (set `self.Target` _asbp_enemy_base)
  (set `self.bPaintDamage` true))

(event `self.BladeCollider.OnComponentEndOverlap`
  (params (OverlappedComponent :type "PrimitiveComponent Object Reference") (OtherActor :type "Actor Object Reference") (OtherComp :type "PrimitiveComponent Object Reference") (OtherBodyIndex :type Integer))
  ;[1 1 1] End Paint Damage on overlap
  (set `self.bPaintDamage` false)
  (set `self.Target` null))

(fn `UserConstructionScript`
  (`parent.UserConstructionScript`))