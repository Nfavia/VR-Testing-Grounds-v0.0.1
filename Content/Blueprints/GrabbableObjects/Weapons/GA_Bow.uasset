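; Grabbable bow weapon, apparently for VR motion controllers, with a two-segment bowstring and no draw or firing logic in this graph.
; The construction script finds the midpoint between the upper and lower string connections and runs each string segment from its connection to that point.
; Gripping the root mesh records the gripping controller as the primary holder, unless a valid one is already set.
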(event `self.ReceiveBeginPlay`
  (`parent.ReceiveBeginPlay`))

(event `self.GrippableMeshRoot.OnGripped`
  (params (GrippingController :type "GripMotionControllerComponent Object Reference") (GripInformation :type "BPActorGripInformation Structure (by ref)"))
  (`self.PrimaryHoldingController`
    (:`then`)
    (:`else`
      (set `self.PrimaryHoldingController` GrippingController))))

(fn `UserConstructionScript`
  (bind _relativelocation (`SceneComponent.RelativeLocation` (`self.LowerStringConnection`)))
  (bind _relativelocation_2 (`SceneComponent.RelativeLocation` (`self.UpperStringConnection`)))
  (`parent.UserConstructionScript`)
  (set `self.StringMidPoint` (+ _relativelocation (* (/ (`KismetMathLibrary.Vector_Distance` _relativelocation _relativelocation_2) 2.0) (`KismetMathLibrary.GetForwardVector` (`KismetMathLibrary.FindLookAtRotation` _relativelocation _relativelocation_2)))))
  (`|ExecutionSequence`
    (:`then_0`
      (`SplineMeshComponent.SetStartAndEnd` (`self.UpperString`) (`SceneComponent.RelativeLocation` (`self.UpperStringConnection`)) (0.0 0.0 0.0) (`self.StringMidPoint`) (0.0 0.0 0.0) true))
    (:`then_1`
      (`SplineMeshComponent.SetStartAndEnd` (`self.LowerSting`) (`SceneComponent.RelativeLocation` (`self.LowerStringConnection`)) (0.0 0.0 0.0) (`self.StringMidPoint`) (0.0 0.0 0.0) true))))